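; SuperPool is an object pool of collectibles that scroll along negative X, likely super pickups for a side-scroller.
; CreateSuper spawns collectibles at the start X with random height and time-scaled random speed until the pool reaches its cap.
; UpdateSupers moves each by its speed per call, recycling those past the opposite edge to the start with new height and speed.
; The event graph is empty, so both functions rely on external callers.
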(event EventBeginPlay)

(event Collision|EventActorBeginOverlap
  (params (OtherActor :type Actor%20Object%20Reference)))

(event EventTick
  (params (DeltaSeconds :type Float%20%28single-precision%29)))

(fn ConstructionScript)

(fn UpdateSupers
  (for (_array_element _array_index) (Variables|Default|GetsuperPool)
    (LocalVariables|SetarrayElement _array_element)
    (LocalVariables|SetarrayIndex _array_index)
    (if (< (.X (Math|Vector|BreakVector (Transformation|GetWorldLocation (Variables|/Script/Engine.Actor|GetRootComponent _array_element)))) (- 0.0 (Variables|Default|GetsStartX)))
      (Transformation|SetWorldLocation (Variables|/Script/Engine.Actor|GetRootComponent (LocalVariables|GetarrayElement)) (Math|Vector|MakeVector (Variables|Default|GetsStartX) 0.0 (Math|Random|RandomFloatinRange -1e+02 5e+02)) false false)
      (bind _ascollectible__ (Utilities|Casting|CastTocollectible++ (LocalVariables|GetarrayElement)))
      (Variables|/Game/Blueprints/collectible++.collectible++_C|SetSpeed _ascollectible__ (Math|Random|RandomFloatinRange 5.0 25.0))
      (else
        (bind _ascollectible___2 (Utilities|Casting|CastTocollectible++ _array_element))
        (Transformation|AddWorldOffset (Variables|/Script/Engine.Actor|GetRootComponent _array_element) (Math|Vector|MakeVector (- 0.0 (Variables|/Game/Blueprints/collectible++.collectible++_C|GetSpeed _ascollectible___2)) 0.0 0.0) false false)))))

(fn CreateSuper
  (if (< (Variables|Default|GetnumberofSuper) (Variables|Default|GetmaxNumberofSuper))
    (bind _returnvalue (Game|SpawnActorfromClass "/Game/Blueprints/collectible++.collectible++_C" (Math|Transform|MakeTransform (Math|Vector|MakeVector (Variables|Default|GetsStartX) 0.0 (Math|Random|RandomFloatinRange -1e+02 5e+02))) "Undefined" 0 0))
    (Variables|/Game/Blueprints/collectible++.collectible++_C|SetSpeed _returnvalue (Math|Random|RandomFloatinRange (/ (Variables|/Game/Blueprints/collectible++.collectible++_C|GetSpeed _returnvalue) (/ (Utilities|Time|GetGameTimeinSeconds) 1e+01)) (Variables|/Game/Blueprints/collectible++.collectible++_C|GetSpeed _returnvalue)))
    (Utilities|Array|Insert (Variables|Default|GetsuperPool) _returnvalue (Variables|Default|GetnumberofSuper))
    (Math|Integer|IncrementInt (Variables|Default|GetnumberofSuper))))