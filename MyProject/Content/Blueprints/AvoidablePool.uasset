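; AvoidablePool is an object pool for Avoidable actors that scroll along negative X, exposed as functions since its event graph is empty.
; CreateAvoidable spawns random classes at AStartX and random height up to a cap, randomizing speed with a time-based lower bound.
; UpdateAvoidables shifts each pooled actor by its Speed per call.
; Actors passing the mirrored X bound are recycled to the start with new random height and speed, avoiding respawns.
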(event EventBeginPlay)

(event Collision|EventActorBeginOverlap
  (params (OtherActor :type Actor%20Object%20Reference)))

(event EventTick
  (params (DeltaSeconds :type Float%20%28single-precision%29)))

(fn ConstructionScript)

(fn CreateAvoidable
  (bind _avoidables (Variables|Default|Getavoidables))
  (if (< (Variables|Default|GetnumberofAvoidables) (Variables|Default|GetmaxNumberofAvoidables))
    (bind _returnvalue (Game|SpawnActorfromClass (Utilities|Array|Get(acopy) _avoidables (Math|Random|RandomIntegerinRange 0 (Utilities|Array|LastIndex _avoidables))) (Math|Transform|MakeTransform (Math|Vector|MakeVector (Variables|Default|GetaStartX) 0.0 (Math|Random|RandomFloatinRange -3e+02 5e+02))) "Undefined" 0))
    (bind _asavoidable (Utilities|Casting|CastToAvoidable _returnvalue))
    (Variables|/Game/Blueprints/Avoidable.Avoidable_C|SetSpeed _asavoidable (Math|Random|RandomFloatinRange (/ (/ (Utilities|Time|GetGameTimeinSeconds) 1e+01) (Variables|/Game/Blueprints/Avoidable.Avoidable_C|GetSpeed _asavoidable)) (Variables|/Game/Blueprints/Avoidable.Avoidable_C|GetSpeed _asavoidable)))
    (Utilities|Array|Insert (Variables|Default|GetthePool) _asavoidable (Variables|Default|GetnumberofAvoidables))
    (Math|Integer|IncrementInt (Variables|Default|GetnumberofAvoidables))))

(fn UpdateAvoidables
  (for (_array_element _array_index) (Variables|Default|GetthePool)
    (LocalVariables|SetarrayElement _array_element)
    (LocalVariables|SetarrayIndex _array_index)
    (if (< (.X (Math|Vector|BreakVector (Transformation|GetWorldLocation (Variables|/Script/Engine.Actor|GetRootComponent _array_element)))) (- 0.0 (Variables|Default|GetaStartX)))
      (Transformation|SetWorldLocation (Variables|/Script/Engine.Actor|GetRootComponent (LocalVariables|GetarrayElement)) (Math|Vector|MakeVector (Variables|Default|GetaStartX) 0.0 (Math|Random|RandomFloatinRange -3e+02 5e+02)) false false)
      (bind _asavoidable (Utilities|Casting|CastToAvoidable (LocalVariables|GetarrayElement)))
      (Variables|/Game/Blueprints/Avoidable.Avoidable_C|SetSpeed _asavoidable (Math|Random|RandomFloatinRange 1e+01 25.0))
      (else
        (bind _asavoidable_2 (Utilities|Casting|CastToAvoidable _array_element))
        (Transformation|AddWorldOffset (Variables|/Script/Engine.Actor|GetRootComponent _array_element) (Math|Vector|MakeVector (- 0.0 (Variables|/Game/Blueprints/Avoidable.Avoidable_C|GetSpeed _asavoidable_2)) 0.0 0.0) false false)))))