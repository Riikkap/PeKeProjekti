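; GainMoreLife is an effect actor that restores the player character's LifeForce when its ApplyEffect event runs.
; If LifeForce is below full, it adds an amount scaled from its Effect value and elapsed game time, capped at the maximum.
; The heal therefore grows the longer the game has run.
; Whenever it heals, it also sets its own Speed to a fixed value.
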(event EventBeginPlay
  (|CallParentFunction) ; This node is disabled and will not be called.\nDrag off pins to build functionality.
)

(event Collision|EventActorBeginOverlap
  (params (OtherActor :type Actor%20Object%20Reference))
  (|CallParentFunction OtherActor) ; This node is disabled and will not be called.\nDrag off pins to build functionality.
)

(event EventApplyEffect
  (params (player%20character :type BB%20Character%20Object%20Reference))
  ;[1 1 1] Onko lifeforce < täydet?
  (if (< (Variables|/Game/Blueprints/BB_Character.BB_Character_C|GetlifeForce player%20character) 1.0)
    ;[1 1 1] Meneekö lifeforce+efekti maksimin yli?
    (if (<= (+ (Variables|/Game/Blueprints/BB_Character.BB_Character_C|GetlifeForce player%20character) (* (/ (Utilities|Time|GetGameTimeinSeconds) 5.0) (* (Variables|Default|GetEffect) 1.5))) 1.0)
      (Variables|/Game/Blueprints/BB_Character.BB_Character_C|SetlifeForce player%20character (+ (Variables|/Game/Blueprints/BB_Character.BB_Character_C|GetlifeForce player%20character) (* (/ (Utilities|Time|GetGameTimeinSeconds) 5.0) (* (Variables|Default|GetEffect) 1.5))))
      (else
        (Variables|/Game/Blueprints/BB_Character.BB_Character_C|SetlifeForce player%20character 1.0)))
    (Variables|Default|SetSpeed 5e+02)))

(event EventTick
  (params (DeltaSeconds :type Float%20%28single-precision%29))
  (|CallParentFunction DeltaSeconds) ; This node is disabled and will not be called.\nDrag off pins to build functionality.
)

(fn ConstructionScript
  (|CallParentFunction))