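; Collectible Blueprint that restores LifeForce to the BB_Character when that character overlaps its Box.
; The overlap event matches the actor's display name, casts it to BB_Character and acts only while LifeForce is below 1.0.
; The gain is Effect multiplied by a factor that grows with elapsed game time, with the result capped at 1.0.
; The graph does not destroy or disable the collectible afterwards.
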(event OnComponentBeginOverlap(Box)
  (params (OverlappedComponent :type Primitive%20Component%20Object%20Reference) (OtherActor :type Actor%20Object%20Reference) (OtherComp :type Primitive%20Component%20Object%20Reference) (OtherBodyIndex :type Integer) (bFromSweep :type Boolean) (SweepResult :type Hit%20Result%20Structure%20%28by%20ref%29))
  ;[1 1 1] Osuuko hahmoon?
  (if (Utilities|Enum|Equal(Enum) (Utilities|GetDisplayName OtherActor) "BB_Character")
    (bind _asbb_character (Utilities|Casting|CastToBB_Character OtherActor))
    ;[1 1 1] Onko lifeforce < täydet?
    (if (< (Variables|/Game/Blueprints/BB_Character.BB_Character_C|GetlifeForce _asbb_character) 1.0)
      ;[1 1 1] Meneekö lifeforce+efekti maksimin yli?
      (if (<= (+ (Variables|/Game/Blueprints/BB_Character.BB_Character_C|GetlifeForce _asbb_character) (* (/ (Utilities|Time|GetGameTimeinSeconds) 5.0) (Variables|Default|GetEffect))) 1.0)
        (Variables|/Game/Blueprints/BB_Character.BB_Character_C|SetlifeForce _asbb_character (+ (Variables|/Game/Blueprints/BB_Character.BB_Character_C|GetlifeForce _asbb_character) (* (/ (Utilities|Time|GetGameTimeinSeconds) 5.0) (Variables|Default|GetEffect))))
        (else
          (Variables|/Game/Blueprints/BB_Character.BB_Character_C|SetlifeForce _asbb_character 1.0))))))

(fn ConstructionScript)