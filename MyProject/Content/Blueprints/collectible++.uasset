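; Collectible pickup Blueprint with a box trigger, apparently intended to restore the BB_Character's LifeForce.
; On overlap it matches the actor by display name, casts it and checks whether LifeForce is below full, but does nothing further.
; The disconnected healing logic would add Effect scaled by elapsed game time, capping LifeForce at full, so the pickup currently has no effect.
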(event OnComponentBeginOverlap(Box)
  (params (OverlappedComponent :type Primitive%20Component%20Object%20Reference) (OtherActor :type Actor%20Object%20Reference) (OtherComp :type Primitive%20Component%20Object%20Reference) (OtherBodyIndex :type Integer) (bFromSweep :type Boolean) (SweepResult :type Hit%20Result%20Structure%20%28by%20ref%29))
  (if (Utilities|Enum|Equal(Enum) (Utilities|GetDisplayName OtherActor) "BB_Character")
    (bind _asbb_character (Utilities|Casting|CastToBB_Character OtherActor))
    (if (< (Variables|/Game/Blueprints/BB_Character.BB_Character_C|GetlifeForce _asbb_character) 1.0)
      _)))

(fn ConstructionScript)