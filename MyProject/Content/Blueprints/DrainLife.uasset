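; DrainLife is an effect actor that reduces a player character's LifeForce when its ApplyEffect event runs.
; The loss is LifeDrain multiplied by a fraction of total game time, so later hits drain more, and LifeForce floors at zero.
; ApplyEffect also sets Speed to a fixed value, while BeginPlay, overlap and Tick are disabled stubs here.
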(event EventBeginPlay)

(event Collision|EventActorBeginOverlap
  (params (OtherActor :type Actor%20Object%20Reference))
  (|CallParentFunction OtherActor) ; This node is disabled and will not be called.\nDrag off pins to build functionality.
)

(event EventTick
  (params (DeltaSeconds :type Float%20%28single-precision%29)))

(event EventApplyEffect
  (params (PlayerCharacter :type BB%20Character%20Object%20Reference))
  (if (> (- (Variables|/Game/Blueprints/BB_Character.BB_Character_C|GetlifeForce PlayerCharacter) (* (/ (Utilities|Time|GetGameTimeinSeconds) 5.0) (Variables|Default|GetlifeDrain))) 0.0)
    (Variables|/Game/Blueprints/BB_Character.BB_Character_C|SetlifeForce PlayerCharacter (- (Variables|/Game/Blueprints/BB_Character.BB_Character_C|GetlifeForce PlayerCharacter) (* (/ (Utilities|Time|GetGameTimeinSeconds) 5.0) (Variables|Default|GetlifeDrain))))
    (else
      (Variables|/Game/Blueprints/BB_Character.BB_Character_C|SetlifeForce PlayerCharacter 0.0)))
  (Variables|Default|SetSpeed 5e+02))

(fn ConstructionScript
  (|CallParentFunction))